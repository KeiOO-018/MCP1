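; Melee enemy that chases and attacks the player, returns to its spawn point after losing sight, and reports to its owning room.
; A self-rescheduling Think loop combines line of sight with a view cone plus an all-around range to choose attack, chase or return.
; Montage notifies open a swing window where Tick sweeps the right fist between frames, damaging the player once per swing.
; Incoming damage reduces HP, destroying it at zero.
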(event `Think`
  (bind _returnvalue (`KismetSystemLibrary.GetGameTimeInSeconds`))
  (bind _homelocation (`self.HomeLocation`))
  (bind _playerref (`self.PlayerRef`))
  (bind _homearriveradius (`self.HomeArriveRadius`))
  (bind _returnvalue_2 (`self.GetDistanceTo` _playerref))
  (bind _returnvalue_3 (`KismetMathLibrary.VSize` (- _homelocation (`self.K2_GetActorLocation`))))
  (`/Engine/EditorBlueprintResources/StandardMacros.IsValid` _playerref
    (:`Is Valid`
      (if (and (`Controller.LineOfSightTo` (`self.GetController`) _playerref (0.0 0.0 0.0) false) (or (<= _returnvalue_2 (`self.ReturnSightRange`)) (and (<= _returnvalue_2 (`self.SightRange`)) (<= (`KismetMathLibrary.DegAcos` (`self.GetHorizontalDotProductTo` _playerref)) (`self.SightHalfAngle`)))))
        (set `self.LastSeenTime` _returnvalue)
        (if (<= _returnvalue_2 (`self.AttackRange`))
          (`Controller.StopMovement` (`self.GetController`))
          (bind _notifyname (`|PlayMontage` (`self.Mesh`) (`self.AttackMontage`))
            (:`then`
              (`KismetSystemLibrary.Delay` (`self.AttackCooldown`))
              (`self.Think`))
            (:`OnBlendOut`
              (set `self.bIsSwinging` false :!label _label))
            (:`OnInterrupted`
              (goto _label))
            (:`OnNotifyBegin`
              (if (== _notifyname "EnemyAttackHit")
                (set `self.bIsSwinging` true)
                (`KismetArrayLibrary.Array_Clear` (`self.HitActorsThisSwing`))
                (set `self.PrevFistCenter` (`SceneComponent.GetSocketLocation` (`self.Mesh`) "HandGrip_R"))))
            (:`OnNotifyEnd`
              (if (== _notifyname "EnemyAttackHit")
                (goto _label))))
          (else
            (`AIBlueprintHelperLibrary.SimpleMoveToActor` (`self.GetController`) _playerref)
            (`KismetSystemLibrary.Delay` (`self.ThinkInterval`))
            (`self.Think`)))
        (elif (and (>= (- _returnvalue (`self.LastSeenTime`)) (`self.ReturnDelay`)) (> _returnvalue_3 _homearriveradius))
          (`AIBlueprintHelperLibrary.SimpleMoveToLocation` (`self.GetController`) _homelocation)
          (`KismetSystemLibrary.Delay` (`self.ThinkInterval`))
          (`self.Think`)
          (elif (<= _returnvalue_3 _homearriveradius)
            (`Controller.StopMovement` (`self.GetController`))
            (`self.K2_SetActorRotation` (`self.HomeRotation`))
            (`KismetSystemLibrary.Delay` (`self.ThinkInterval`))
            (`self.Think`)
            (else
              (`Controller.StopMovement` (`self.GetController`))
              (`KismetSystemLibrary.Delay` (`self.ThinkInterval`))
              (`self.Think`))))))
    (:`Is Not Valid`
      (set `self.PlayerRef` (`GameplayStatics.GetPlayerCharacter` 0))
      (`KismetSystemLibrary.Delay` (`self.ThinkInterval`))
      (`self.Think`))))

(event `self.ReceiveTick`
  (params (DeltaSeconds :type "Float (single-precision)"))
  (if (`self.bIsSwinging`)
    (bind _outhits (`KismetSystemLibrary.SphereTraceMultiForObjects` :`Start` (`self.PrevFistCenter`) :`End` (`SceneComponent.GetSocketLocation` (`self.Mesh`) "HandGrip_R") :`Radius` (`self.FistRadius`) :`ObjectTypes` (`|MakeArray` "ObjectTypeQuery3" :!type "EObjectTypeQuery Enum") :`DrawTime` 0.5))
    (for _array_element _outhits
      (bind (_bblockinghit _binitialoverlap _time _distance _location _impactpoint _normal _impactnormal _physmat _hitactor) (`GameplayStatics.BreakHitResult` _array_element))
      (if (not (`KismetArrayLibrary.Array_Contains` (`self.HitActorsThisSwing`) _hitactor))
        (`KismetArrayLibrary.Array_Add` (`self.HitActorsThisSwing`) _hitactor)
        (if (== _hitactor (`self.PlayerRef`))
          (`GameplayStatics.ApplyDamage` _hitactor (`self.AttackDamage`) (`self.GetController`) self))))
    (set `self.PrevFistCenter` (`SceneComponent.GetSocketLocation` (`self.Mesh`) "HandGrip_R"))))

(event `self.ReceiveBeginPlay`
  (bind _owningroom (`self.OwningRoom`))
  (set `self.PlayerRef` (`GameplayStatics.GetPlayerCharacter` 0))
  (set `self.HomeLocation` (`self.K2_GetActorLocation`))
  (set `self.HomeRotation` (`self.K2_GetActorRotation`))
  (set `self.LastSeenTime` (`KismetSystemLibrary.GetGameTimeInSeconds`))
  (set `self.CurrentHP` (`self.MaxHP`))
  (`/Engine/EditorBlueprintResources/StandardMacros.IsValid` _owningroom
    (:`Is Valid`
      (`/Game/Progression/BP_StageRoom.RegisterEnemy` _owningroom self))
    (:`Is Not Valid`
      _))
  (`self.Think`))

(event `self.ReceiveAnyDamage`
  (params (Damage :type "Float (single-precision)") (DamageType :type "DamageType Object Reference") (InstigatedBy :type "Controller Object Reference") (DamageCauser :type "Actor Object Reference"))
  (bind _owningroom (`self.OwningRoom`))
  (bind _output_get (set `self.CurrentHP` (`KismetMathLibrary.FClamp` (- (`self.CurrentHP`) Damage) 0.0 (`self.MaxHP`))))
  (`KismetSystemLibrary.PrintString` (`KismetStringLibrary.Concat_StrStr` "EnemyHP: " (`KismetStringLibrary.Conv_DoubleToString` _output_get)))
  (if (<= _output_get 0.0)
    (`/Engine/EditorBlueprintResources/StandardMacros.IsValid` _owningroom
      (:`Is Valid`
        (`/Game/Progression/BP_StageRoom.NotifyEnemyDied` _owningroom))
      (:`Is Not Valid`
        _))
    (`self.K2_DestroyActor`)))

(fn `UserConstructionScript`)