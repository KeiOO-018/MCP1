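; BP_Door is an interactable hinged door that can be locked behind a required key.
; Interact on a locked door asks BP_ThirdPersonCharacter to consume the selected key, then unlocks and toggles, or shows a locked message on failure.
; Toggling eases the Hinge between closed and OpenAngle over a time set by SwingSpeed.
; The construction script offsets the mesh by its Y scale to put the hinge on either side.
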(event `ToggleDoor`
  (bind _output_get (set `self.bOpen` (not (`self.bOpen`))))
  (`KismetSystemLibrary.MoveComponentTo` (`self.Hinge`) (0.0 0.0 0.0) (`KismetMathLibrary.MakeRotator` 0.0 0.0 (`KismetMathLibrary.SelectFloat` (`self.OpenAngle`) 0.0 _output_get)) true true (/ 1.0 (`self.SwingSpeed`))))

(event `/Game/Interaction/BPI_Interact.Interact`
  (params (Interactor :type "Actor Object Reference"))
  (if (`self.bLocked`)
    (bind _asbp_third_person_character (cast `/Game/ThirdPerson/Blueprints/BP_ThirdPersonCharacter` Interactor))
    (bind _success (`/Game/ThirdPerson/Blueprints/BP_ThirdPersonCharacter.TryConsumeSelected` _asbp_third_person_character (`.RowName` (break `DataTableRowHandle` (`self.RequiredKey`)))))
    (if _success
      (set `self.bLocked` false)
      (`self.ToggleDoor` :!label _label)
      (else
        (`/Game/ThirdPerson/Blueprints/BP_ThirdPersonCharacter.ShowHUDMessage` _asbp_third_person_character "DOOR IS LOCKED")))
    (else
      (goto _label))))

(fn `UserConstructionScript`
  (`SceneComponent.K2_SetRelativeLocation` (`self.DoorMesh`) (`KismetMathLibrary.MakeVector` 0.0 (* (* 100.0 (.y (`SceneComponent.RelativeScale3D` (`self.DoorMesh`)))) (select `bool` (`self.bHingeOnRight`) :`false` 1.0 :`true` -1.0))) false false))