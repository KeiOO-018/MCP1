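; BP_StageRoom tracks the living enemies in a stage room and rewards the player when the room is cleared.
; RegisterEnemy and NotifyEnemyDied raise and lower the EnemiesAlive counter, with no Tick or overlap logic.
; When the count reaches zero, a final room shows "STAGE CLEAR" through BP_ThirdPersonCharacter's HUD message.
; Any other room spawns a BP_ItemPickup at DropPoint, using KeyToDrop as its item row.
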(fn `NotifyEnemyDied`
  (set `self.EnemiesAlive` (- (`self.EnemiesAlive`) 1))
  (if (== (`self.EnemiesAlive`) 0)
    (if (`self.bIsFinalRoom`)
      (bind _asbp_third_person_character (cast `/Game/ThirdPerson/Blueprints/BP_ThirdPersonCharacter` (`GameplayStatics.GetPlayerCharacter` 0)))
      (`/Game/ThirdPerson/Blueprints/BP_ThirdPersonCharacter.ShowHUDMessage` _asbp_third_person_character "STAGE CLEAR")
      (else
        (`|SpawnActorFromClass` "/Game/Inventory/BP_ItemPickup.BP_ItemPickup_C" (`KismetMathLibrary.MakeTransform` (`SceneComponent.K2_GetComponentLocation` (`self.DropPoint`))) "AlwaysSpawn" "MultiplyWithRoot" null (`self.KeyToDrop`) null)))))

(fn `RegisterEnemy`
  (set `self.EnemiesAlive` (+ (`self.EnemiesAlive`) 1)))

(fn `UserConstructionScript`)